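; BP_Enemy is a patrolling enemy that kills BP_Player on overlap by calling its Die function.
; On BeginPlay it stores the actor's world location as StartPosition, then loops MoveComponentTo on its StaticMesh over MoveTime, alternating between EndPosition and StartPosition.
; Both points are passed as relative-location targets, although StartPosition comes from world space.
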(event `self.ReceiveBeginPlay`
  ;[1 1 1] Enemy patrol moving
  (set `self.StartPosition` (`self.K2_GetActorLocation`))
  (set `self.TargetPosition` (`self.EndPosition`))
  (`KismetSystemLibrary.MoveComponentTo` (`self.StaticMesh`) (`self.TargetPosition`) (struct) false false (`self.MoveTime`) :!label _label)
  (if (== (`self.TargetPosition`) (`self.StartPosition`))
    (set `self.TargetPosition` (`self.EndPosition`))
    (goto _label)
    (else
      (set `self.TargetPosition` (`self.StartPosition`))
      (goto _label))))

(event `self.ReceiveActorBeginOverlap`
  (params (OtherActor :type "Actor Object Reference"))
  ;[1 1 1] Kill player on touch
  (bind _asbp_player (cast `/Game/Blueprints/BP_Player` OtherActor))
  (`/Game/Blueprints/BP_Player.Die` _asbp_player))

(fn `UserConstructionScript`)